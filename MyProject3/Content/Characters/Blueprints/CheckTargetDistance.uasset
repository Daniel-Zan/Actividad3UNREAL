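; Behavior tree decorator that checks whether the AI's pawn is within an acceptable distance of its follow target.
; It compares the straight-line distance between the controlled pawn and the TargetToFollow blackboard actor against AcceptableDistance.
; A successful cast of the owner to MyAIController only caches the reference.
; The distance result returns on the cast-failed branch, using that cached reference.
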(fn PerformConditionCheck
  (params (OwnerActor :type Actor%20Object%20Reference))
  (bind _asmy_aicontroller (Utilities|Casting|CastToMyAIController OwnerActor)
    (:then
      (Variables|Default|SetAICtrlRef _asmy_aicontroller))
    (:CastFailed
      (return (<= (Math|Vector|VectorLength (- (Transformation|GetActorLocation (AI|BehaviorTree|GetBlackboardValueasActor (Variables|Default|GetTargetToFollow))) (Transformation|GetActorLocation (Pawn|GetControlledPawn (Variables|Default|GetAICtrlRef))))) (Variables|Default|GetAcceptableDistance))))))